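; Enemy creature that chases the player, optionally staying hidden and without collision until Aparecer is called.
; Aparecer reveals it and starts a looping timer on Perseguir, which re-issues a simple AI move toward the player and checks capture by distance.
; On capture it stops the timer, disables player input, shows a caught message through WBP_Mensaje and loads LVL_Test after a delay.
; Tick plays or stops the mesh animation based on movement speed.
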(event Custom|Perseguir
  (bind _returnvalue (Game|GetPlayerController 0))
  (bind _returnvalue_2 (Game|GetPlayerCharacter 0))
  (AI|Navigation|SimpleMovetoActor (Pawn|GetController) _returnvalue_2)
  (if (and (< (Transformation|GetDistanceTo _returnvalue_2) 1.2e+02) (not (Variables|Default|GetAtrapado)))
    (Variables|Default|SetAtrapado true)
    (Utilities|Time|ClearTimerbyFunctionName self "Perseguir")
    (Input|DisableInput _returnvalue_2 _returnvalue)
    (bind _returnvalue_3 (UserInterface|CreateWidget "/Game/BackrUms/UI/WBP_Mensaje.WBP_Mensaje_C" _returnvalue))
    (Rendering|Components|TextRender|SetText (Variables|/Game/BackrUms/UI/WBP_Mensaje.WBP_Mensaje_C|GetTextoMensaje _returnvalue_3) "TE ATRAPARON")
    (UserInterface|Viewport|AddtoViewport _returnvalue_3 0)
    (Utilities|FlowControl|Delay 3.0)
    (Game|OpenLevel(byName) "LVL_Test")))

(event Custom|Aparecer
  (Rendering|SetActorHiddenInGame false)
  (Collision|SetActorEnableCollision true)
  (Utilities|Time|SetTimerbyFunctionName self "Perseguir" 0.5 true))

(event EventBeginPlay
  (Variables|/Script/Engine.CharacterMovementComponent|SetMaxWalkSpeed (Variables|Character|GetCharacterMovement) (Variables|Default|GetVelocidad))
  (if (Variables|Default|GetOcultaAlInicio)
    (Rendering|SetActorHiddenInGame true)
    (Collision|SetActorEnableCollision false)))

(event Collision|EventActorBeginOverlap
  (params (OtherActor :type Actor%20Object%20Reference)))

(event EventTick
  (params (DeltaSeconds :type Float%20%28single-precision%29))
  (bind _charactermovement (Variables|Character|GetCharacterMovement))
  (bind _velocity (Variables|/Script/Engine.MovementComponent|GetVelocity _charactermovement))
  (bind _returnvalue (Math|Vector|VectorLength _velocity))
  (bind _returnvalue_2 (> _returnvalue 1e+01))
  (if (and _returnvalue_2 (not (Variables|Default|GetAnimando)))
    (Audio|Components|Audio|Play (Variables|Character|GetMesh) true)
    (Variables|Default|SetAnimando true)
    (elif (and (not _returnvalue_2) (Variables|Default|GetAnimando))
      (Audio|Components|Audio|Stop (Variables|Character|GetMesh))
      (Variables|Default|SetAnimando false))))

(fn ConstructionScript)